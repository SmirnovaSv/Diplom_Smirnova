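; Enemy turret that tracks the nearest visible player character in sensing range and can fire bullets from twin barrels.
; Each tick it picks a target by sphere overlap and line of sight, then turns its top at constant speed with clamped pitch.
; UpdateFire gates Fire by rate and dot-product aim, though nothing here calls it.
; Fire spawns left then right bullets at sockets, using delays and a DoN gate.
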(event `self.ReceiveTick`
  (params (DeltaSeconds :type "Float (single-precision)"))
  ;[1 1 1] Поиск цели
  (`self.FindBestTarget`)
  (`self.Target`
    (:`then`
      ;[1 1 1] Вращение башни турели
      (`self.UpdateTurretRotation` DeltaSeconds))
    (:`else`)))

(event `Fire`
  (set `self.Time Of Last Fire` (`KismetSystemLibrary.GetGameTimeInSeconds`))
  (`|ExecutionSequence`
    (:`then_0`
      (goto _label :!via `Reset`))
    (:`then_1`
      (`/Engine/EditorBlueprintResources/StandardMacros.Do N` 2 :!label _label
        (:`Exit`
          (`|SpawnActorFromClass` "/Game/Survive/Enemy/Turret/Bullet.Bullet_C" (`SceneComponent.GetSocketTransform` (`self.Barrel_L`) "FireSocket" "RTS_World") "Undefined" "OverrideRootScale" null null)
          (`KismetSystemLibrary.Delay` 0.2)
          (`|SpawnActorFromClass` "/Game/Survive/Enemy/Turret/Bullet.Bullet_C" (`SceneComponent.GetSocketTransform` (`self.Barrel_R`) "FireSocket" "RTS_World") "Undefined" "OverrideRootScale" null null)
          (`KismetSystemLibrary.Delay` 0.2)
          (goto _label :!via `Reset`))))))

(fn `FindBestTarget`
  (locals (`Best Distance (Local)` :type "Float (double-precision)") (`Current Distance (Local)` :type "Float (double-precision)") (`Best Target (Local)` :type "Actor Object Reference") (`Current Target (Local)` :type "Actor Object Reference"))
  (set `local.Best Distance (Local)` (+ (`self.Sensing Range`) 1.0))
  (bind _outactors (`KismetSystemLibrary.SphereOverlapActors` (`self.K2_GetActorLocation`) (`self.Sensing Range`) (`|MakeArray` "ObjectTypeQuery3" :!type "EObjectTypeQuery Enum") "/Game/ThirdPersonBP/Blueprints/ThirdPersonCharacter.ThirdPersonCharacter_C"))
  (for _array_element _outactors
    (bind _output_get (set `local.Current Target (Local)` _array_element))
    (bind _output_get_2 (set `local.Current Distance (Local)` (`self.GetDistanceTo` _output_get self)))
    ;[1 1 1] Это ближайшая цель на данный момент?
    (if (or (< _output_get_2 (`local.Best Distance (Local)`)) (not (`KismetSystemLibrary.IsValid` (`local.Best Target (Local)`))))
      (bind _result (`/Game/MyFunctionLibrary.HasLineOfSight` (`SceneComponent.K2_GetComponentLocation` (`self.Top`)) (`self.K2_GetActorLocation` (`local.Current Target (Local)`)) (`|MakeArray` self (`local.Current Target (Local)`) :!type "Actor Object Reference")))
      (if _result
        (set `local.Best Target (Local)` (`local.Current Target (Local)`))
        (set `local.Best Distance (Local)` (`local.Current Distance (Local)`)))))
  (set `self.Target` (`local.Best Target (Local)`)))

(fn `UpdateFire`
  ;[1 1 1] Сеижение скорострельности?
  (if (> (- (`KismetSystemLibrary.GetGameTimeInSeconds`) (`self.Time Of Last Fire`)) (`self.Rate of Fire`))
    ;[1 1 1] Направлена ли турель на цель?
    (if (> (`KismetMathLibrary.Dot_VectorVector` (`KismetMathLibrary.GetDirectionUnitVector` (`SceneComponent.K2_GetComponentLocation` (`self.Top`)) (`self.K2_GetActorLocation` (`self.Target`))) (`SceneComponent.GetForwardVector` (`self.Top`))) 0.99)
      (`self.Fire`))))

(fn `UpdateTurretRotation`
  (params (`Delta Seconds` :type "Float (double-precision)"))
  (locals (`New Rotation` :type "Rotator Structure" :default (struct)))
  (bind _output_get (set `local.New Rotation` (`KismetMathLibrary.RInterpTo_Constant` (`SceneComponent.K2_GetComponentRotation` (`self.Top`)) (`KismetMathLibrary.FindLookAtRotation` (`SceneComponent.K2_GetComponentLocation` (`self.Top`)) (`self.K2_GetActorLocation` (`self.Target`))) (`local.Delta Seconds`) (`self.Rotation Speed`))))
  (`SceneComponent.K2_SetWorldRotation` (`self.Top`) (`KismetMathLibrary.MakeRotator` (.roll _output_get) (`KismetMathLibrary.ClampAngle` (.pitch _output_get) -45.0 75.0) (.yaw _output_get)) false false))

(fn `UserConstructionScript`)