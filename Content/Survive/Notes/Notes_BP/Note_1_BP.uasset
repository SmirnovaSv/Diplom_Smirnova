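; Note_1_BP is a readable note pickup that shows a Note_Wiget on screen when the player presses F nearby.
; Box overlap enables input and opens a gate; F then flip-flops between showing the widget with the Cube hidden and removing it with the Cube visible.
; Leaving the Box disables input, removes the widget and restores the Cube, without closing the gate or resetting the FlipFlop.
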(event `Key|F`
  (params (Key :type "Key Structure"))
  (bind _cube (`self.Cube`))
  (:`Pressed`
    (`/Engine/EditorBlueprintResources/StandardMacros.Gate` true :!label _label
      (:`Exit`
        (`/Engine/EditorBlueprintResources/StandardMacros.FlipFlop`
          (:`A`
            (bind _returnvalue (`|CreateWidget` "/Game/Survive/Notes/WidGet/Note_Wiget.Note_Wiget_C"))
            (`UserWidget.AddToViewport` _returnvalue 0)
            (`SceneComponent.SetVisibility` _cube false false))
          (:`B`
            (`Widget.RemoveFromParent` _returnvalue :!label _label_2)
            (`SceneComponent.SetVisibility` _cube true false)))))))

(event `self.Box.OnComponentBeginOverlap`
  (params (OverlappedComponent :type "PrimitiveComponent Object Reference") (OtherActor :type "Actor Object Reference") (OtherComp :type "PrimitiveComponent Object Reference") (OtherBodyIndex :type Integer) (bFromSweep :type Boolean) (SweepResult :type "HitResult Structure (by ref)"))
  (`self.EnableInput` (`GameplayStatics.GetPlayerController` 0))
  (goto _label :!via `Open`))

(event `self.Box.OnComponentEndOverlap`
  (params (OverlappedComponent :type "PrimitiveComponent Object Reference") (OtherActor :type "Actor Object Reference") (OtherComp :type "PrimitiveComponent Object Reference") (OtherBodyIndex :type Integer))
  (`self.DisableInput` (`GameplayStatics.GetPlayerController` 0))
  (goto _label_2))

(fn `UserConstructionScript`)