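; Essence_BP holds the player life system's four vitals: health, stamina, hunger and thirst.
; BeginPlay fills each vital to its maximum.
; ValueLoss subtracts a loss amount from a passed-in value, floors the result at zero and returns it without storing it.
; Tick is empty, and nothing in this Blueprint calls ValueLoss or drains the vitals over time.
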(event `self.ReceiveBeginPlay`
  (set `self.Health` (`self.Max Health`))
  (set `self.Stamina` (`self.Max Stamina`))
  (set `self.Hunger` (`self.Max Hunger`))
  (set `self.Thirst` (`self.Max Thirst`)))

(event `self.ReceiveTick`
  (params (DeltaSeconds :type "Float (single-precision)")))

(fn `Value Loss`
  (params (`Parameter Type` :type "Float (double-precision)") (`Loss Amount` :type "Float (double-precision)"))
  (returns (`Parameter Result` :type "Float (double-precision)"))
  (bind _returnvalue (- `Parameter Type` `Loss Amount`))
  (return (`KismetMathLibrary.SelectFloat` 0.0 _returnvalue (< _returnvalue 0.0))))